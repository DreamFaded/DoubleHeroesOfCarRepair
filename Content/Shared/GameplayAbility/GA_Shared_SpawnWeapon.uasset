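; Shared gameplay ability that spawns a weapon actor for its avatar and attaches it to the character.
; On activation it spawns the configured weapon class with the avatar as owner and instigator, then attaches it to the owning component at a configurable socket.
; It registers the weapon with the pawn combat component under a gameplay tag, optionally as equipped, and ends once the spawn succeeds.
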(event `self.K2_ActivateAbility`
  (bind _returnvalue (`self.GetAvatarActorFromActorInfo`))
  (bind _returnvalue_2 (`|SpawnActorFromClass` (`self.WeaponClassToSpawn`) (`KismetMathLibrary.MakeTransform` (0.0 0.0 0.0)) "AdjustIfPossibleButAlwaysSpawn" "MultiplyWithRoot" _returnvalue (cast `Pawn` _returnvalue :!pure true)))
  (`/Engine/EditorBlueprintResources/StandardMacros.IsValid` _returnvalue_2
    (:`Is Valid`
      (`Actor.K2_AttachToComponent` _returnvalue_2 (`self.GetOwningComponentFromActorInfo`) (`self.SocketNameToAttachTo`) "SnapToTarget" "KeepRelative" "KeepWorld" true)
      (`PawnCombatComponent.RegisterSpawnedWeapon` (`self.GetPawnCombatComponentFromActorInfo`) (`self.WeaponTagToRegister`) _returnvalue_2 (`self.Register as Equipped Weapon`))
      (`self.K2_EndAbility`))))
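; GA_Hero_LightAttack_Master is the hero's light attack gameplay ability, cycling through a montage combo chain.
; Each activation clears the pending reset timer, plays the montage mapped to the current combo count, then advances the count, wrapping after the last entry.
; When the montage completes, blends out or is interrupted or cancelled, the ability ends and starts a short timer that resets the combo to the first attack.
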(event `self.K2_ActivateAbility`
  (`KismetSystemLibrary.K2_ClearAndInvalidateTimerHandle` (`self.ComboCountResetTimerHandle`))
  (`AbilityTask_PlayMontageAndWait.CreatePlayMontageAndWaitProxy` "None" (`BlueprintMapLibrary.Map_Find` (`self.AttackMontagesMap`) (`self.CurrentLightAttackComboCount`))
    (:`then`
      (`|ExecutionSequence`
        (:`then_0`
          (if (== (`self.CurrentLightAttackComboCount`) (`BlueprintMapLibrary.Map_Length` (`self.AttackMontagesMap`)))
            (`self.ResetAttackComboCount`)
            (else
              (`/Engine/EditorBlueprintResources/StandardMacros.IncrementInt` (`self.CurrentLightAttackComboCount`)))))))
    (:`OnCompleted`
      (`self.K2_EndAbility` :!label _label)
      (bind _returnvalue (`KismetSystemLibrary.K2_SetTimerDelegate` (delegate `ResetAttackComboCount`) 1.0))
      (set `self.ComboCountResetTimerHandle` _returnvalue))
    (:`OnBlendOut`
      (goto _label))
    (:`OnInterrupted`
      (goto _label))
    (:`OnCancelled`
      (goto _label))))

(event `ResetAttackComboCount`
  (set `self.CurrentLightAttackComboCount` 1))
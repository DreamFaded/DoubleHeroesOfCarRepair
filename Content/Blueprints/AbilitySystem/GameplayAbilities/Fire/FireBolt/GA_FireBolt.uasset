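; GA_FireBolt is the Fire Bolt gameplay ability: it casts a projectile toward the point under the mouse.
; On activation, a target-data task gets the cursor hit location, then turns the avatar to face it through CombatInterface.
; It plays the throw montage and waits for the montage's gameplay event, so the projectile spawns on a specific keyframe.
; After spawning, it ends following a short delay.
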(event `self.K2_ActivateAbility`
  (bind (_asynctaskproxy _datahandle) (`TargetDataUnderMouse.CreateTargetDataUnderMouse`)
    (:`ValidData`
      (set `self.ProjectileTargetLocation` (`.Location` (`GameplayStatics.BreakHitResult` (`AbilitySystemBlueprintLibrary.GetHitResultFromTargetData` _datahandle))))
      (bind _ascombat_interface (cast `CombatInterface` (`self.GetAvatarActorFromActorInfo`)))
      (`CombatInterface.UpdateFacingTarget` _ascombat_interface (`self.ProjectileTargetLocation`))
      (`AbilityTask_PlayMontageAndWait.CreatePlayMontageAndWaitProxy` "None" "/Game/Animations/FightingAnimsetPro/AM_Cast_Throw.AM_Cast_Throw"
        (:`then`
          ;[1 1 1] 物体在指定关键帧发射
          (`AbilityTask_WaitGameplayEvent.WaitGameplayEvent` (struct :`TagName` "Event.Montage.FireBolt") null
            (:`EventReceived`
              (`self.SpawnProjectile` (`self.ProjectileTargetLocation`))
              (`KismetSystemLibrary.Delay` 0.5)
              (`self.K2_EndAbility`))))))))
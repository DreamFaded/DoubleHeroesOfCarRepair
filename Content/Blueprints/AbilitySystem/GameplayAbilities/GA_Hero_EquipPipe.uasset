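; GA_Hero_EquipPipe is a hero gameplay ability holding the logic for equipping a weapon, named for the pipe.
; HandleEquipWeapon caches the weapon's hero data, then links its animation layer and adds its Enhanced Input mapping context.
; It grants the weapon's default abilities at the ability's level and stores the returned spec handles on the weapon.
; ActivateAbility is empty, and nothing in this file calls HandleEquipWeapon.
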(event `self.K2_ActivateAbility`)

(fn `HandleEquipWeapon`
  (params (InWeaponToEquip :type "DoubleHeroesWeapon Object Reference"))
  (locals (CachedHeroWeaponData :type "DoubleHeroesWeaponData Structure" :default (struct :`WeaponAnimLayerToLink` "/Script/Engine.AnimBlueprintGeneratedClass'\"/Game/Blueprints/Character/AnimBP/AnimLayer/AnimLayer_BlueHeroPipe.AnimLayer_BlueHeroPipe_C\"'" :`DefaultWeaponAbilities` "(())")))
  (set `local.CachedHeroWeaponData` (`DoubleHeroesWeapon.HeroesWeaponData` InWeaponToEquip))
  (`|ExecutionSequence`
    (:`then_0`
      (`SkeletalMeshComponent.LinkAnimClassLayers` (`self.GetOwningComponentFromActorInfo`) (`.WeaponAnimLayerToLink` (break `DoubleHeroesWeaponData` (`local.CachedHeroWeaponData`)))))
    (:`then_1`
      (`EnhancedInputSubsystemInterface.AddMappingContext` (pcsubsystem `EnhancedInputLocalPlayerSubsystem` (`self.GetHeroControllerFromActorInfo`)) (`.WeaponInputMappingContext` (break `DoubleHeroesWeaponData` (`local.CachedHeroWeaponData`))) 1 (struct)))
    (:`then_2`
      (bind _outgrantedabilityspechandles (`DHAbilitySystemComponent.GrantHeroWeaponAbilities` (`self.GetDHAbilitySystemComponentFromActorInfo`) (`.DefaultWeaponAbilities` (break `DoubleHeroesWeaponData` (`local.CachedHeroWeaponData`))) (`self.GetAbilityLevel`)))
      (`DoubleHeroesWeapon.AssignGrantedAbilitySpecHandles` (`local.InWeaponToEquip`) _outgrantedabilityspechandles))))
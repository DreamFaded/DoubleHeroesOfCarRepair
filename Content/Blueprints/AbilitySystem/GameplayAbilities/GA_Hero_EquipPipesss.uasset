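; Hero gameplay ability that equips the carried FireBowl weapon while playing a one-handed sword equip montage.
; On the montage's equip gameplay event, it attaches the weapon to RightHandSocket and records it as equipped in the combat component.
; HandleEquipWeapon uses the weapon's data to link anim layers, add an input mapping context and grant weapon abilities, storing their handles on the weapon.
; The ability ends when the montage completes, blends out, or is interrupted or cancelled.
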(event `self.K2_ActivateAbility`
  (`AbilityTask_PlayMontageAndWait.CreatePlayMontageAndWaitProxy` "None" "/Game/Animations/FightingAnimsetPro/Montages/AM_Sword1h_Equip_Montage.AM_Sword1h_Equip_Montage"
    (:`then`
      (`AbilityTask_WaitGameplayEvent.WaitGameplayEvent` (struct :`TagName` "Player.Event.Equip.FireBowl") null
        (:`EventReceived`
          (`Actor.K2_AttachToComponent` (`PawnCombatComponent.GetCharacterCarriedWeaponByTag` (`self.GetHeroCombatComponentFromActorInfo`) (struct :`TagName` "Player.Weapon.FireBowl")) (`self.GetOwningComponentFromActorInfo`) "RightHandSocket" "SnapToTarget" "KeepRelative" "KeepWorld" true)
          (`self.HandleEquipWeapon` (`HeroCombatComponent.GetHeroCarriedWeaponByTag` (`self.GetHeroCombatComponentFromActorInfo`) (struct :`TagName` "Player.Weapon.FireBowl")))
          (set `PawnCombatComponent.CurrentEquippedWeaponTag` (struct :`TagName` "Player.Weapon.FireBowl") (`self.GetHeroCombatComponentFromActorInfo`)))))
    (:`OnCompleted`
      (`self.K2_EndAbility` :!label _label))
    (:`OnBlendOut`
      (goto _label))
    (:`OnInterrupted`
      (goto _label))
    (:`OnCancelled`
      (goto _label))))

(fn `HandleEquipWeapon`
  (params (InWeaponToEquip :type "DoubleHeroesWeapon Object Reference"))
  (locals (CachedHeroWeaponData :type "DoubleHeroesWeaponData Structure"))
  (set `local.CachedHeroWeaponData` (`DoubleHeroesWeapon.HeroesWeaponData` InWeaponToEquip))
  (`|ExecutionSequence`
    (:`then_0`
      (`SkeletalMeshComponent.LinkAnimClassLayers` (`self.GetOwningComponentFromActorInfo`) (`.WeaponAnimLayerToLink` (break `DoubleHeroesWeaponData` (`local.CachedHeroWeaponData`)))))
    (:`then_1`
      (`EnhancedInputSubsystemInterface.AddMappingContext` (pcsubsystem `EnhancedInputLocalPlayerSubsystem` (`self.GetHeroControllerFromActorInfo`)) (`.WeaponInputMappingContext` (break `DoubleHeroesWeaponData` (`local.CachedHeroWeaponData`))) 1 (struct)))
    (:`then_2`
      (bind _outgrantedabilityspechandles (`DHAbilitySystemComponent.GrantHeroWeaponAbilities` (`self.GetDHAbilitySystemComponentFromActorInfo`) (`.DefaultWeaponAbilities` (break `DoubleHeroesWeaponData` (`local.CachedHeroWeaponData`))) (`self.GetAbilityLevel`)))
      (`DoubleHeroesWeapon.AssignGrantedAbilitySpecHandles` (`local.InWeaponToEquip`) _outgrantedabilityspechandles))))
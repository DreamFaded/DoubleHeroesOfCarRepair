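; GA_Crouch is a gameplay ability that crouches the avatar Character while the input is held.
; Activation caches the ASC and Character, applies the GE_Crouch effect, calls Crouch and waits for input release.
; On release, a WaitCrouchClearance task with sphere-trace parameters holds the ability active until there is clearance to stand, then ends it.
; Ending uncrouches the character, removes the effect by its stored handle and cleans up both async tasks.
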(event `self.K2_ActivateAbility`
  (`self.CacheEssentialVars`)
  (`self.ApplyCrouchEffect`)
  (`Character.Crouch` (`self.AvatarCharacter`))
  (bind _asynctaskproxy (`AbilityTask_WaitInputRelease.WaitInputRelease` false)
    (:`then`
      (set `self.WaitInputReleaseAsyncTask` _asynctaskproxy))
    (:`OnRelease`
      (bind _asynctaskproxy_2 (`AbilityTask_WaitCrouchClearance.WaitCrouchClearance` 90.0 35.0 true)
        (:`then`
          (set `self.CrouchClearanceAsyncTask` _asynctaskproxy_2))
        (:`HasClearance`
          (`self.K2_EndAbility`))))))

(event `self.K2_OnEndAbility`
  (params (bWasCancelled :type Boolean))
  (`Character.UnCrouch` (`self.AvatarCharacter`))
  (`self.BP_RemoveGameplayEffectFromOwnerWithHandle` (`self.ActiveCouchEffect`))
  (`self.CleanupAsyncTasks`))

(fn `ApplyCrouchEffect`
  (bind _owningasc (`self.OwningASC`))
  (bind _returnvalue (`AbilitySystemComponent.BP_ApplyGameplayEffectSpecToSelf` (`self.OwningASC`) (`AbilitySystemComponent.MakeOutgoingSpec` _owningasc "/Game/Blueprints/AbilitySystem/GameplayEffects/GE_Crouch.GE_Crouch_C" 0.0 (`AbilitySystemComponent.MakeEffectContext` _owningasc))))
  (set `self.ActiveCouchEffect` _returnvalue))

(fn `CacheEssentialVars`
  (set `self.OwningASC` (`self.GetAbilitySystemComponentFromActorInfo`))
  (bind _ascharacter (cast `Character` (`self.GetAvatarActorFromActorInfo`)))
  (set `self.AvatarCharacter` _ascharacter))

(fn `CleanupAsyncTasks`
  (bind _crouchclearanceasynctask (`self.CrouchClearanceAsyncTask`))
  (bind _waitinputreleaseasynctask (`self.WaitInputReleaseAsyncTask`))
  (`/Engine/EditorBlueprintResources/StandardMacros.IsValid` _waitinputreleaseasynctask
    (:`Is Valid`
      (`GameplayTask.EndTask` _waitinputreleaseasynctask))
    (:`Is Not Valid`
      _))
  (`/Engine/EditorBlueprintResources/StandardMacros.IsValid` _crouchclearanceasynctask
    (:`Is Valid`
      (`GameplayTask.EndTask` _crouchclearanceasynctask))))